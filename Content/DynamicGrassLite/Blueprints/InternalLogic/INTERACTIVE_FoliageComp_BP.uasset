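; Interactive foliage component from DynamicGrassLite that declares an API for per-instance deformation, offsets and status tracking, such as trampling.
; It covers starting offsets, querying deform and un-deform alphas, copying foliage parameters and editing instance statuses.
; Every function here is a stub that does nothing or returns a default value.
; BeginPlay and EndPlay only call the parent, and Tick is disabled.
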(event Custom|DivideIntoChunks_InfLoopWorkaround
  (params (chunkSize :type Float%20%28single-precision%29)))

(event EventBeginPlay
  (|CallParentFunction))

(event EventTick
  (params (DeltaSeconds :type Float%20%28single-precision%29)))

(event EventEndPlay
  (params (EndPlayReason :type EEndPlayReason%20Enum :default "Destroyed"))
  (|CallParentFunction EndPlayReason))

(fn StartNewInstanceOffset
  (params (Instance :type Integer) (NewOffset :type Vector) (DeformDuration :type Float%20%28single-precision%29) (UnDeformSpeed :type Float%20%28single-precision%29) (UpdateComponent :type Boolean) (IgnoreIfGrowing :type Float%20%28single-precision%29)))

(fn ForceMarkDirty)

(fn GetCurrentInstanceUN-DeformAlpha
  (params (InstanceIndex :type Integer))
  (return false 0.0))

(fn GetCurrentInstanceGPUOffset
  (params (InstanceIndex :type Integer) (AtSpecifiedAlpha :type Boolean) (SpecifiedAlpha :type Float%20%28single-precision%29))
  (return ""))

(fn GetCurrentInstanceDeformAlpha
  (params (InstanceIndex :type Integer))
  (return false 0.0))

(fn Copy&SetFoliageParametersfromClass
  (params (copyFrom :type INTERACTIVE%20Foliage%20Comp%20BP%20Class%20Reference) (meshToSet :type Static%20Mesh%20Object%20Reference)))

(fn Copy&SetFoliageParameters
  (params (copyFrom :type INTERACTIVE%20Foliage%20Comp%20BP%20Object%20Reference)))

(fn RemoveAnyActiveStatuses
  (params (InstanceIndex :type Integer)))

(fn IsTrampled?
  (params (instanceIndex :type Integer))
  (return false))

(fn RemoveInstanceStatus
  (params (instanceIndex :type Integer) (Status :type InstanceStatus%20Enum :default "NewEnumerator0")))

(fn AddInstanceStatus
  (params (instanceIndex :type Integer) (Status :type InstanceStatus%20Enum :default "NewEnumerator0")))